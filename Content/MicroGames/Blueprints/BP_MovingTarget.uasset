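; BP_MovingTarget is a micro-game target that patrols back and forth and can be destroyed by hits.
; A looping timer negates Direction every MovementDuration, while Tick offsets the actor along it by Speed per frame, unscaled by delta time and without sweep.
; Each hit spawns an explosion effect and sound, decrementing HitPoints or, if already at zero or below, destroying the actor with a different sound.
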(event Custom|CustomEvent_FlipDirection
  ;[1 1 1] Flip Direction
  (Variables|Default|SetDirection (* (Variables|Default|GetDirection) -1.0)))

(event EventBeginPlay
  ;[1 1 1] Flip Direction
  (Utilities|Time|SetTimerbyEvent (delegate Custom|CustomEvent_FlipDirection) (Variables|Default|GetMovementDuration) true))

(event EventTick
  (params (DeltaSeconds :type Float%20%28single-precision%29))
  ;[1 0.5248 0.7308] Target Movement
  (Transformation|AddActorWorldOffset (* (Math|Vector|Normalize (Variables|Default|GetDirection)) (Variables|Default|GetSpeed))))

(event Collision|EventHit
  (params (MyComp :type Primitive%20Component%20Object%20Reference) (Other :type Actor%20Object%20Reference) (OtherComp :type Primitive%20Component%20Object%20Reference) (bSelfMoved :type Boolean) (HitLocation :type Vector :default "0, 0, 0") (HitNormal :type Vector :default "0, 0, 0") (NormalImpulse :type Vector :default "0, 0, 0") (Hit :type Hit%20Result%20Structure%20%28by%20ref%29))
  ;[1 0.9276 0.5412] TargetHit
  (if (<= (Variables|Default|GetHitPoints) 0)
    ;[0.2325 1 0.7673] Destroy
    (Effects|SpawnEmitteratLocation "/Game/StarterContent/Particles/P_Explosion.P_Explosion" HitLocation)
    (Audio|PlaySoundatLocation "/Game/StarterContent/Audio/Explosion02.Explosion02" HitLocation "0, 0, 0" 1.0 1.0 0.0 0 0 0 0)
    (Actor|DestroyActor)
    (else
      (Variables|Default|SetHitPoints (- (Variables|Default|GetHitPoints) 1))
      (Effects|SpawnEmitteratLocation "/Game/StarterContent/Particles/P_Explosion.P_Explosion" HitLocation)
      (Audio|PlaySoundatLocation "/Game/StarterContent/Audio/Explosion01.Explosion01" HitLocation "0, 0, 0" 1.0 1.0 0.0 0 0 0 0))))

(fn ConstructionScript)
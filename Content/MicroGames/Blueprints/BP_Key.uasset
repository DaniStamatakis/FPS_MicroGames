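; BP_Key is a key pickup that appears once no BP_MovingTarget actors remain in the level.
; Each tick it checks the target array, toggles mesh visibility and collision, and fires a one-time explosion effect and sound on reveal.
; When the player character overlaps its sphere collider after the reveal, it sets HasKey on that character, plays a sound and destroys itself.
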(event OnComponentBeginOverlap(Sphere_Collider)
  (params (OverlappedComponent :type Primitive%20Component%20Object%20Reference) (OtherActor :type Actor%20Object%20Reference) (OtherComp :type Primitive%20Component%20Object%20Reference) (OtherBodyIndex :type Integer) (bFromSweep :type Boolean) (SweepResult :type Hit%20Result%20Structure%20%28by%20ref%29))
  ;[0.3904 0.8284 1] Key - Pickup & Destroy
  (if (and (== OtherActor (Variables|Default|GetAs%20BP%20First%20Person%20Character)) (Variables|Default|GetAllTargetsDestroyed))
    (Variables|/Game/FirstPerson/Blueprints/BP_FirstPersonCharacter.BP_FirstPersonCharacter_C|SetHasKey (Variables|Default|GetAs%20BP%20First%20Person%20Character) true)
    (Audio|PlaySoundatLocation "/Game/StarterContent/Audio/Explosion01.Explosion01" (Transformation|GetActorLocation) "0, 0, 0" 1.0 1.0 0.0 0 0 0 0)
    (Actor|DestroyActor)))

(event EventBeginPlay
  ;[1 0.622 0.5654] Getting the Player Reference
  (bind _asbp_first_person_character (Utilities|Casting|CastToBP_FirstPersonCharacter (Game|GetPlayerCharacter 0)))
  (Variables|Default|SetAs%20BP%20First%20Person%20Character _asbp_first_person_character))

(event EventTick
  (params (DeltaSeconds :type Float%20%28single-precision%29))
  (bind _sm_key (Variables|Default|GetSM_Key))
  (bind _returnvalue (Transformation|GetWorldLocation _sm_key))
  ;[1 0.683 0.9325] Key - Visbility
  (bind _outactors (Actor|GetAllActorsOfClass "/Game/MicroGames/Blueprints/BP_MovingTarget.BP_MovingTarget_C"))
  (bind _returnvalue_2 (Utilities|Array|Add _outactors 0))
  (bind _output_get (Variables|Default|SetAllTargetsDestroyed (<= _returnvalue_2 0)))
  (Rendering|SetVisibility (Variables|Default|GetSM_Key) _output_get true)
  (Collision|SetActorEnableCollision _output_get)
  ;[0.6211 0.5111 1] Key - Spawn Effects
  (if (Variables|Default|GetAllTargetsDestroyed)
    (Utilities|FlowControl|DoOnce false
      (:Completed
        (Effects|SpawnEmitteratLocation "/Game/StarterContent/Particles/P_Explosion.P_Explosion" _returnvalue)
        (Audio|PlaySoundatLocation "/Game/StarterContent/Audio/Collapse01.Collapse01" _returnvalue "0, 0, 0" 1.0 1.0 0.0 0 0 0 0)))))

(fn ConstructionScript)